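; BP_Footsteps is an animation notify that plays a footstep sound from the animated skeletal mesh.
; It spawns the configured sound attached to the mesh at a named bone, with an adjustable volume multiplier.
; It then passes the notify's Type as the integer parameter FootstepType on the spawned audio component, so the sound asset can vary by step type.
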(fn ReceivedNotify
  (params (MeshComp :type Skeletal%20Mesh%20Component%20Object%20Reference) (Animation :type Anim%20Sequence%20Base%20Object%20Reference))
  (Utilities|IsValid (Variables|Default|GetSoundWave)
    (:Is%20Valid
      (bind _returnvalue (Audio|SpawnSoundAttached (Variables|Default|GetSoundWave) MeshComp (Variables|Default|GetBoneName) "0, 0, 0" "0, 0, 0" "KeepRelativeOffset" false (Variables|Default|GetVolumeMultiplier) 1.0 0.0 0 0))
      (Utilities|IsValid _returnvalue
        (:Is%20Valid
          (Effects|Components|ParticleSystem|SetIntParameter _returnvalue "FootstepType" (Math|Conversions|ToInteger(Byte) (Variables|Default|GetType)))
          (return true))
        (:Is%20Not%20Valid
          (return true))))))