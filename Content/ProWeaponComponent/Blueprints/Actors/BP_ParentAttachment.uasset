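; Base actor for weapon attachments that mounts itself on its owning BP_Weapon in the ProWeaponComponent system.
; On BeginPlay it finds the DT_Attachments row whose ParentClass matches its own class and stores that row's attachment type.
; It then attaches to the owner's WeaponMesh at AttachBoneName, keeping relative transforms.
; A multicast event plays a given sound attached to its root.
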(event Custom|PlaySound%20%28%20MULTICAST%20%29
  (params (Sound :type Sound%20Base%20Object%20Reference))
  (Audio|SpawnSoundAttached Sound (Variables|Default|GetDefaultSceneRoot) "None" "0, 0, 0" "0, 0, 0" "KeepRelativeOffset" false 1.0 1.0 0.0 "/Game/ProWeaponComponent/Assets/SoundSettings/SA_Realistic.SA_Realistic" 0))

(event EventBeginPlay
  ;[0 0 0] Begin Play - Read Data and Attach To Parent Weapon
  (CallFunction|ReadData)
  (CallFunction|AttachtoParent))

(fn ConstructionScript)

(fn AttachtoParent
  ;[0 0 0] Attach Attachment To Parent Weapon
  (Utilities|IsValid (Components|GetOwner)
    (:Is%20Valid
      (bind _asbp_weapon (Utilities|Casting|CastToBP_Weapon (Components|GetOwner))
        (:then
          (Transformation|AttachComponentToComponent self (Variables|/Game/ProWeaponComponent/Blueprints/Actors/BP_Weapon.BP_Weapon_C|GetWeaponMesh _asbp_weapon) (Variables|Default|GetAttachBoneName) "KeepRelative" "KeepRelative" "KeepRelative" true)
          (return))
        (:CastFailed
          (return))))
    (:Is%20Not%20Valid
      (return))))

(fn ReadData
  ;[0 0 0] Takes Attachment Info From Datatable
  (bind _outrownames (DataTable|GetDataTableRowNames "/Game/ProWeaponComponent/Blueprints/Datatables/Attachments/DT_Attachments.DT_Attachments"))
  (for _array_element _outrownames
    (bind _returnvalue (Utilities|GetDataTableRow "/Game/ProWeaponComponent/Blueprints/Datatables/Attachments/DT_Attachments.DT_Attachments" _array_element)
      (:then
        (if (== (.ParentClass (Utilities|Struct|BreakS_Attachment _returnvalue)) (Utilities|GetClass self))
          (Variables|Default|SetType (.AttachmentType (Utilities|Struct|BreakS_Attachment _returnvalue)))
          (return)))))
  (return))