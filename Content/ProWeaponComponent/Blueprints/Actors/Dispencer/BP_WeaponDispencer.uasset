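; Weapon dispenser pickup that displays a slowly spinning weapon mesh, looked up by ID from the weapons DataTable in construction and on BeginPlay.
; A looping timer advances the target yaw, and Tick interpolates the mesh toward it.
; Box overlap plays a pickup sound, updates the HUD and calls a server event.
; That event adds the weapon unless the actor's current weapon shares the ID, optionally auto-equipping it.
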(event OnComponentBeginOverlap(Box)
  (params (OverlappedComponent :type Primitive%20Component%20Object%20Reference) (OtherActor :type Actor%20Object%20Reference) (OtherComp :type Primitive%20Component%20Object%20Reference) (OtherBodyIndex :type Integer) (bFromSweep :type Boolean) (SweepResult :type Hit%20Result%20Structure%20%28by%20ref%29))
  ;[0 0 0] On Overlap Add Weapon By ID
  (CallFunction|AddWeapon(SERVER) OtherActor)
  (Audio|SpawnSoundatLocation "/Game/ProWeaponComponent/Assets/Sounds/Impacts/SN_Pickup.SN_Pickup" (Transformation|GetActorLocation) "0, 0, 0" 1.0 1.0 0.0 (CallFunction|GetSoundAttenuation) 0)
  (Utilities|FlowControl|Delay 0.1)
  (Class|BPIWCHUD|UpdateWeapons(Message) (CallFunction|GetWCHUD)))

(event Custom|AddRotation
  ;[0 0 0] Rotation Mesh
  (Variables|Default|SetRotation (+ (Variables|Default|GetRotation) 3.0)))

(event Custom|AddWeapon%20%28%20SERVER%20%29
  (params (Target :type Object%20Object%20Reference))
  ;[0 0 0] On Overlap Add Weapon By ID
  (CallFunction|AddFunction Target))

(event EventBeginPlay
  ;[0 0 0] Rotation Mesh
  (CallFunction|SetWeaponMesh)
  (Utilities|Time|SetTimerbyEvent (delegate Custom|AddRotation) 0.1 true))

(event EventTick
  (params (DeltaSeconds :type Float%20%28single-precision%29))
  ;[0 0 0] Rotation Mesh
  (Transformation|SetRelativeRotation (Variables|Default|GetWeapon) (Math|Interpolation|RInterpTo (Variables|/Script/Engine.SceneComponent|GetRelativeRotation (Variables|Default|GetWeapon)) (Math|Rotator|MakeRotator 0.0 0.0 (Variables|Default|GetRotation)) (Utilities|Time|GetWorldDeltaSeconds) 2.0) false false))

(fn ConstructionScript
  (CallFunction|SetWeaponMesh))

(fn SetWeaponMesh
  ;[0 0 0] Read Weapon Mesh From Datatable
  (bind _outrownames (DataTable|GetDataTableRowNames (CallFunction|GetUsingWeaponsDatatable)))
  (bind _returnvalue (Utilities|GetDataTableRow (CallFunction|GetUsingWeaponsDatatable) (Utilities|Array|Get(acopy) _outrownames (Variables|Default|GetID)))
    (:then
      (Class|SkinnedMeshComponent|SetSkeletalMesh (Variables|Default|GetWeapon) (.SkeletalMesh (Utilities|Struct|BreakS_WeaponDesign (.Design (Utilities|Struct|BreakS_Weapon _returnvalue)))) true)
      (return))
    (:RowNotFound
      (return))))

(fn AddFunction
  (params (Target :type Object%20Object%20Reference))
  ;[0 0 0] Check Is Valid Weapon Component
  (bind _weaponcomponent (Class|BPIGetWeaponComponent|GetWeaponComponent(Message) Target))
  (bind _output_get (LocalVariables|SetlWeaponComponent _weaponcomponent))
  (Utilities|IsValid _output_get
    (:Is%20Valid
      ;[0 0 0] Check Has Current Weapon
      (Utilities|IsValid (Default|GetCurrentWeapon (LocalVariables|GetlWeaponComponent))
        (:Is%20Valid
          (if (!= (Variables|/Game/ProWeaponComponent/Blueprints/Actors/BP_Weapon.BP_Weapon_C|GetID (Default|GetCurrentWeapon (LocalVariables|GetlWeaponComponent))) (Variables|Default|GetID))
            _
            (else
              (return))))
        (:Is%20Not%20Valid
          _))
      ;[0 0 0] Add Weapon And AutoEquip
      (bind (_success _index) (Default|SpawnandAddWeapon (LocalVariables|GetlWeaponComponent) (Variables|Default|GetID) (Variables|Default|GetToIndex) (Variables|Default|GetAmmo) (Variables|Default|GetlEmpty)))
      (if (and _success (Variables|Default|GetbAutoEquip))
        (Variables|/Game/ProWeaponComponent/Blueprints/Components/BPC_WeaponComponent.BPC_WeaponComponent_C|SetbSwapWeapons (LocalVariables|GetlWeaponComponent) false)
        (Default|EquipWeapon(SERVER) (LocalVariables|GetlWeaponComponent) _index)
        (return)
        (else
          (return))))
    (:Is%20Not%20Valid
      (return))))