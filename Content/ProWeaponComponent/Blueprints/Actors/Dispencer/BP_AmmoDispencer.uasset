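; Ammo dispenser actor that grants a fixed amount of ammo for its configured ID to an actor overlapping its box.
; The overlap calls a server event that gets the target's weapon component through GetWeaponComponentMessage and adds the ammo.
; A pickup sound plays on every overlap, and the dispenser is never consumed.
; A looping timer advances a target yaw, which Tick interpolates toward to spin the Ammo component smoothly.
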(event OnComponentBeginOverlap(Box)
  (params (OverlappedComponent :type Primitive%20Component%20Object%20Reference) (OtherActor :type Actor%20Object%20Reference) (OtherComp :type Primitive%20Component%20Object%20Reference) (OtherBodyIndex :type Integer) (bFromSweep :type Boolean) (SweepResult :type Hit%20Result%20Structure%20%28by%20ref%29))
  ;[0 0 0] On Overlap Add Ammo By ID
  (CallFunction|AddWeapon(SERVER) OtherActor)
  (Audio|SpawnSoundatLocation "/Game/ProWeaponComponent/Assets/Sounds/Impacts/SN_Pickup.SN_Pickup" (Transformation|GetActorLocation) "0, 0, 0" 1.0 1.0 0.0 (CallFunction|GetSoundAttenuation) 0))

(event Custom|AddRotation
  ;[0 0 0] Rotation Mesh
  (Variables|Default|SetRotation (+ (Variables|Default|GetRotation) 3.0)))

(event Custom|AddWeapon%20%28%20SERVER%20%29
  (params (Target :type Object%20Object%20Reference))
  ;[0 0 0] On Overlap Add Ammo By ID
  (bind _weaponcomponent (Class|BPIGetWeaponComponent|GetWeaponComponent(Message) Target))
  (Utilities|IsValid _weaponcomponent
    (:Is%20Valid
      (Default|AddAmmobyID _weaponcomponent (Variables|Default|GetID) 100))))

(event EventBeginPlay
  ;[0 0 0] Rotation Mesh
  (Utilities|Time|SetTimerbyEvent (delegate Custom|AddRotation) 0.1 true))

(event EventTick
  (params (DeltaSeconds :type Float%20%28single-precision%29))
  ;[0 0 0] Rotation Mesh
  (Transformation|SetRelativeRotation (Variables|Default|GetAmmo) (Math|Interpolation|RInterpTo (Variables|/Script/Engine.SceneComponent|GetRelativeRotation (Variables|Default|GetAmmo)) (Math|Rotator|MakeRotator 0.0 0.0 (Variables|Default|GetRotation)) (Utilities|Time|GetWorldDeltaSeconds) 2.0) false false))

(fn ConstructionScript)