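; Helper actor that follows the wielder's look-at point, positioning itself where the aim of its owning weapon attachment lands.
; Each tick it traces from its owner toward the look-at location and interpolates to the hit or far endpoint, destroying itself if the three-level owner chain breaks.
; It falls back to a trace along the owner's negated forward vector when pitch is too steep or during sprint, reload, firing or weapon swap.
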(event EventTick
  (params (DeltaSeconds :type Float%20%28single-precision%29))
  (bind _returnvalue (Components|GetOwner))
  (bind _returnvalue_2 (Components|GetOwner))
  (bind _returnvalue_3 (Components|GetOwner))
  (bind _returnvalue_4 (Components|GetOwner _returnvalue))
  (bind _returnvalue_5 (Transformation|GetActorLocation _returnvalue_3))
  (bind _returnvalue_6 (Transformation|GetActorLocation _returnvalue_2))
  (bind _returnvalue_7 (Components|GetOwner _returnvalue_4))
  (Utilities|IsValid _returnvalue
    (:Is%20Valid
      (Utilities|IsValid _returnvalue_4
        (:Is%20Valid
          (Utilities|IsValid _returnvalue_7
            (:Is%20Valid
              (bind _location (Class|BPIWCCharacter|GetLookatLocation(Message) _returnvalue_7 0.0))
              (bind (_outhit _returnvalue_8) (Collision|LineTraceByChannel (Math|Vector|MakeVector (.x _returnvalue_6) (.y _returnvalue_6) (.Z (Math|Vector|BreakVector (select (and (< (Math|Float|Absolute(Float) (.pitch (Math|Rotator|FindLookatRotation (Transformation|GetActorLocation (Components|GetOwner)) _location))) 12.0) (CallFunction|ShouldDraw)) _location (CallFunction|GetForwardLocation))))) (Math|Vector|MakeVector (.x (+ (* (- (select (and (< (Math|Float|Absolute(Float) (.pitch (Math|Rotator|FindLookatRotation (Transformation|GetActorLocation (Components|GetOwner)) _location))) 12.0) (CallFunction|ShouldDraw)) _location (CallFunction|GetForwardLocation)) _returnvalue_5) 1e+03) _returnvalue_5)) (.y (+ (* (- (select (and (< (Math|Float|Absolute(Float) (.pitch (Math|Rotator|FindLookatRotation (Transformation|GetActorLocation (Components|GetOwner)) _location))) 12.0) (CallFunction|ShouldDraw)) _location (CallFunction|GetForwardLocation)) _returnvalue_5) 1e+03) _returnvalue_5)) (.Z (Math|Vector|BreakVector (select (and (< (Math|Float|Absolute(Float) (.pitch (Math|Rotator|FindLookatRotation (Transformation|GetActorLocation (Components|GetOwner)) _location))) 12.0) (CallFunction|ShouldDraw)) _location (CallFunction|GetForwardLocation))))) "TraceTypeQuery1" false 0 "None"))
              (if _returnvalue_8
                (Transformation|SetActorLocation (Math|Interpolation|VInterpTo (Transformation|GetActorLocation) (.Location (Collision|BreakHitResult _outhit)) (Utilities|Time|GetWorldDeltaSeconds) 1e+02) false true)
                (else
                  (Transformation|SetActorLocation (Math|Interpolation|VInterpTo (Transformation|GetActorLocation) (+ (* (- (select (and (< (Math|Float|Absolute(Float) (.pitch (Math|Rotator|FindLookatRotation (Transformation|GetActorLocation (Components|GetOwner)) _location))) 12.0) (CallFunction|ShouldDraw)) _location (CallFunction|GetForwardLocation)) _returnvalue_5) 1e+03) _returnvalue_5) (Utilities|Time|GetWorldDeltaSeconds) 1e+02) false true))))
            (:Is%20Not%20Valid
              (Actor|DestroyActor :!label _label))))
        (:Is%20Not%20Valid
          (goto _label))))
    (:Is%20Not%20Valid
      (goto _label))))

(fn ConstructionScript)

(fn ShouldDraw
  (bind _bsprint (Class|BPIWCCharacter|GetSprint(Message) (Components|GetOwner (Components|GetOwner (Components|GetOwner)))))
  (if _bsprint
    (return false)
    (else
      (bind _asbp_weapon (Utilities|Casting|CastToBP_Weapon (Components|GetOwner (Components|GetOwner)))
        (:then
          (if (or (Variables|/Game/ProWeaponComponent/Blueprints/Actors/BP_Weapon.BP_Weapon_C|GetbInReload _asbp_weapon) (Variables|/Game/ProWeaponComponent/Blueprints/Actors/BP_Weapon.BP_Weapon_C|GetbInFire _asbp_weapon))
            (return false)
            (else
              (bind _weaponcomponent (Class|BPIGetWeaponComponent|GetWeaponComponent(Message) (Components|GetOwner (Components|GetOwner (Components|GetOwner)))))
              (if (Variables|/Game/ProWeaponComponent/Blueprints/Components/BPC_WeaponComponent.BPC_WeaponComponent_C|GetbSwapWeapons _weaponcomponent)
                (return false)
                (else
                  (return true))))))
        (:CastFailed
          (return false))))))

(fn GetForwardLocation
  (bind _returnvalue (Components|GetOwner))
  (bind _returnvalue_2 (Transformation|GetActorForwardVector _returnvalue))
  (bind _returnvalue_3 (* _returnvalue_2 -1e+05))
  (bind _returnvalue_4 (+ _returnvalue_3 "0, 0, 0"))
  (bind _returnvalue_5 (+ "0, 0, 0" _returnvalue_4))
  (bind (_outhit _returnvalue_6) (Collision|LineTraceByChannel (Transformation|GetWorldLocation (Variables|/Script/Engine.Actor|GetRootComponent _returnvalue)) _returnvalue_5 "TraceTypeQuery1" false 0 "None"))
  (if _returnvalue_6
    (return (.Location (Collision|BreakHitResult _outhit)))
    (else
      (return _returnvalue_5))))