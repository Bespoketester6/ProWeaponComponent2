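; Parent projectile for the weapon component that applies damage, pushes physics objects and can pierce what it hits.
; The server handles hits, multicasting physical-material-based impact effects and the projectile's destruction.
; Piercing reverse-traces for an exit point and respawns the projectile with absorption-scaled damage and speed, carrying hit actors until cumulative absorption falls below a threshold.
; A Ricochet function similarly spawns a mirrored copy, but nothing here calls it.
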(event Custom|Destroy%20%28%20MULTICAST%20%29
  ;[0 0 0] Destroy Projectile
  (Actor|DestroyActor))

(event Custom|Particle%20%28%20MULTICAST%20%29
  (params (Location :type Vector) (Rotation :type Rotator) (EmitterTemplate :type Particle%20System%20Object%20Reference) (Sound :type Sound%20Base%20Object%20Reference))
  ;[0 0 0] Spawn Particle And Sound ( MULTICAST )
  (Audio|SpawnSoundatLocation Sound Location "0, 0, 0" 1.0 1.0 0.0 (CallFunction|GetSoundAttenuation) 0)
  (Effects|SpawnEmitteratLocation EmitterTemplate Location Rotation))

(event Collision|EventHit
  (params (MyComp :type Primitive%20Component%20Object%20Reference) (Other :type Actor%20Object%20Reference) (OtherComp :type Primitive%20Component%20Object%20Reference) (bSelfMoved :type Boolean) (HitLocation :type Vector :default "0, 0, 0") (HitNormal :type Vector :default "0, 0, 0") (NormalImpulse :type Vector :default "0, 0, 0") (Hit :type Hit%20Result%20Structure%20%28by%20ref%29))
  ;[0 0 0] Hit Event
  ;;[0 0 0] Process Hit Only On Server
  (if (Networking|IsServer)
    (if (and (!= Other (Components|GetOwner)) (!= Other (Variables|Links|GetOwningWeapon)))
      ;;[0 0 0] Apply Damage
      (CallFunction|ApplyDamage Other)
      (bind (_particle _sound) (CallFunction|SpawnImpactParicle))
      ;;[0 0 0] Spawn Projectile Particle
      (CallFunction|Particle(MULTICAST) HitLocation (Math|Rotator|MakeRotfromX HitNormal) _particle _sound)
      ;;[0 0 0] Set Hiden Mesh
      (Rendering|SetVisibility (Variables|MyProjectile|GetProjectileMesh) false false)
      ;;[0 0 0] Add Physic Impulse
      (if (Physics|IsSimulatingPhysics OtherComp "None")
        (Physics|AddImpulseatLocation OtherComp (* (Transformation|GetVelocity) 1e+02) (Transformation|GetActorLocation) "None")))
    ;;[0 0 0] Process Projectile Pierce
    (CallFunction|Pierce OtherComp Other)
    ;;[0 0 0] Destroy Projectile
    (CallFunction|Destroy(MULTICAST))))

(fn ConstructionScript
  (bind _projectile (Variables|MyProjectile|GetProjectile))
  ;[0 0 0] Init Projectile
  (bind _output_get (Variables|/Script/Engine.ProjectileMovementComponent|SetMaxSpeed _projectile (Variables|Params|GetSpeed)))
  (Variables|/Script/Engine.ProjectileMovementComponent|SetInitialSpeed _projectile _output_get)
  (Variables|/Script/Engine.ProjectileMovementComponent|SetbShouldBounce _projectile false))

(fn SpawnImpactParicle
  (bind _returnvalue (Transformation|GetActorLocation))
  (bind _outhit (Collision|SphereTraceByChannel _returnvalue _returnvalue 5.0 "TraceTypeQuery1" false 0 "None"))
  (bind _impactsound (CallFunction|PhysicMaterialtoImpactSound (.PhysMat (Collision|BreakHitResult _outhit))))
  (bind _particle (CallFunction|PhysicMaterialtoParticle (.PhysMat (Collision|BreakHitResult _outhit))))
  (return _particle _impactsound))

(fn Pierce
  (params (Component :type Scene%20Component%20Object%20Reference) (Actor :type Actor%20Object%20Reference))
  (bind _returnvalue (Transformation|GetActorLocation))
  (LocalVariables|SetlOverlapedActor Actor)
  (if (Utilities|Array|ContainsItem (Variables|Links|GetHitActors) (LocalVariables|GetlOverlapedActor))
    _
    (else
      (bind _success (Class|BPIPierceActor|CanPierce(Message) (LocalVariables|GetlOverlapedActor)))
      (if (and _success (Variables|Boolean|GetCanPierce))
        (bind _percent (Class|BPIPierceActor|GetImpulseAbsorving(Message) (LocalVariables|GetlOverlapedActor)))
        (LocalVariables|SetlAbsorving _percent)
        (elif (or (== (LocalVariables|GetlOverlapedActor) (Components|GetOwner)) (== (LocalVariables|GetlOverlapedActor) (Variables|Links|GetOwningWeapon)))
          _
          (else
            (return false))))
      (Utilities|Array|AddUnique (Variables|Links|GetHitActors) (LocalVariables|GetlOverlapedActor))))
  (bind _outhits (Collision|MultiLineTraceByChannel (+ _returnvalue (* (Transformation|GetActorForwardVector) 1e+02)) (+ _returnvalue (* (Transformation|GetActorForwardVector) 1e+01)) "TraceTypeQuery1" false 0 "None"))
  (for _array_element _outhits
    (if (or (== (.HitComponent (Collision|BreakHitResult _array_element)) Component) (== (.HitActor (Collision|BreakHitResult _array_element)) (LocalVariables|GetlOverlapedActor)))
      (LocalVariables|SetlNewLocation (.Location (Collision|BreakHitResult _array_element)))
      (if (> (CallFunction|CalcSummaryAbsorving) (Variables|Params|GetSpeedToDestroyPercent))
        (Game|SpawnActorfromClass (Utilities|GetClass self) (Math|Transform|MakeTransform (LocalVariables|GetlNewLocation) (Transformation|GetActorRotation) "1,1,1") "AlwaysSpawn" (Components|GetOwner) (* (Variables|Params|GetDamage) (LocalVariables|GetlAbsorving)) (* (Variables|Params|GetSpeed) (LocalVariables|GetlAbsorving)) (Variables|Params|GetAccuracy) (Variables|Links|GetHitActors) (Variables|Links|GetOwningWeapon) 0)
        (return true)
        (else
          (return false)))))
  (LocalVariables|SetlNewLocation (+ (Transformation|GetActorLocation) (* (Transformation|GetActorForwardVector) 1e+01)))
  (if (> (CallFunction|CalcSummaryAbsorving) (Variables|Params|GetSpeedToDestroyPercent))
    (Game|SpawnActorfromClass (Utilities|GetClass self) (Math|Transform|MakeTransform (LocalVariables|GetlNewLocation) (Transformation|GetActorRotation) "1,1,1") "AlwaysSpawn" (Components|GetOwner) (* (Variables|Params|GetDamage) (LocalVariables|GetlAbsorving)) (* (Variables|Params|GetSpeed) (LocalVariables|GetlAbsorving)) (Variables|Params|GetAccuracy) (Variables|Links|GetHitActors) (Variables|Links|GetOwningWeapon) 0)
    (return true)
    (else
      (return false))))

(fn CalcSummaryAbsorving
  (for _array_element (Variables|Links|GetHitActors)
    (Utilities|IsValid _array_element
      (:Is%20Valid
        (bind _success (Class|BPIPierceActor|CanPierce(Message) _array_element))
        (if _success
          (bind _percent (Class|BPIPierceActor|GetImpulseAbsorving(Message) _array_element))
          (LocalVariables|SetlResult (* _percent (LocalVariables|GetlResult)))))))
  (return (LocalVariables|GetlResult)))

(fn Ricochet
  (params (Normal :type Vector) (Absorving :type Float%20%28single-precision%29) (SpeedLimit :type Float%20%28single-precision%29))
  (if (> (Variables|Params|GetSpeed) SpeedLimit)
    (Game|SpawnActorfromClass (Utilities|GetClass self) (Math|Transform|MakeTransform (Transformation|GetActorLocation) (Math|Rotator|MakeRotfromX (Math|Vector|MirrorVectorbyNormal (Math|Rotator|GetRotationXVector (Transformation|GetActorRotation)) Normal)) "1,1,1") "AlwaysSpawn" (Components|GetOwner) (* (Variables|Params|GetDamage) Absorving) (* (Variables|Params|GetSpeed) Absorving) (Variables|Params|GetAccuracy) (Variables|Links|GetHitActors) (Variables|Links|GetOwningWeapon) 0)
    (return true)
    (else
      (return false))))

(fn ApplyDamage
  (params (Target :type Actor%20Object%20Reference))
  ;[0 0 0] Apply Damage
  (Game|Damage|ApplyDamage Target (Variables|Params|GetDamage) 0 (Components|GetOwner))
  (return))