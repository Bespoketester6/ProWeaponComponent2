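; Shotgun shell projectile that, on BeginPlay on the server, spawns a burst of BP_PierceProjectile pellets carrying its Damage and Speed.
; Pellets aim at the owner's accuracy-based look-at location via BPI_WCCharacter, or otherwise scatter randomly around the forward vector.
; Its Pierce function tracks hit actors, line-traces for a new location and respawns a pierce projectile with absorption-scaled damage and speed if the summed absorption clears a threshold.
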(event EventBeginPlay
  (bind _returnvalue (Components|GetOwner))
  (bind _returnvalue_2 (Transformation|GetActorLocation))
  (bind _returnvalue_3 (Transformation|GetActorLocation))
  (if (Networking|IsServer)
    (for _index (range 0 7)
      (if (Utilities|DoesObjectImplementInterface _returnvalue "/Game/ProWeaponComponent/Blueprints/Interfaces/BPI_WCCharacter.BPI_WCCharacter_C")
        (bind _location (Class|BPIWCCharacter|GetLookatLocation(Message) _returnvalue (Variables|Default|GetAccuracy)))
        (Game|SpawnActorfromClass "/Game/ProWeaponComponent/Blueprints/Actors/Projectiles/BP_PierceProjectile.BP_PierceProjectile_C" (Math|Transform|MakeTransform _returnvalue_2 (Math|Rotator|MakeRotfromX (- _location _returnvalue_2)) "1,1,1") "AlwaysSpawn" (Components|GetOwner) (Variables|Default|GetDamage) (Variables|Default|GetSpeed) 0.0 0 0 0)
        (else
          (Game|SpawnActorfromClass "/Game/ProWeaponComponent/Blueprints/Actors/Projectiles/BP_PierceProjectile.BP_PierceProjectile_C" (Math|Transform|MakeTransform _returnvalue_3 (Math|Rotator|MakeRotfromX (- (+ (* (+ (Transformation|GetActorForwardVector) (* (Math|Random|RandomUnitVector) 0.1)) 1e+02) (Transformation|GetActorLocation)) _returnvalue_3)) "1,1,1") "AlwaysSpawn" (Components|GetOwner) (Variables|Default|GetDamage) (Variables|Default|GetSpeed) 0.0 0 0 0))))))

(fn ConstructionScript
  (|CallParentFunction))

(fn Pierce
  (params (Component :type Scene%20Component%20Object%20Reference) (Actor :type Actor%20Object%20Reference))
  (bind _returnvalue (Transformation|GetActorLocation))
  (LocalVariables|SetlOverlapedActor 0)
  (if (Utilities|Array|ContainsItem (Variables|Default|GetHitActors) (LocalVariables|GetlOverlapedActor))
    _
    (else
      (bind _success (Class|BPIPierceActor|CanPierce(Message) (LocalVariables|GetlOverlapedActor)))
      (if (and _success (Variables|Default|GetCanPierce))
        (bind _percent (Class|BPIPierceActor|GetImpulseAbsorving(Message) (LocalVariables|GetlOverlapedActor)))
        (LocalVariables|SetlAbsorving _percent)
        (elif (== (LocalVariables|GetlOverlapedActor) (Components|GetOwner))
          _
          (else
            (return))))
      (Utilities|Array|AddUnique (Variables|Default|GetHitActors) (LocalVariables|GetlOverlapedActor))))
  (bind _outhits (Collision|MultiLineTraceByChannel (+ _returnvalue (* (Transformation|GetActorForwardVector) 1e+02)) (+ _returnvalue (* (Transformation|GetActorForwardVector) 1e+01)) "TraceTypeQuery1" false 0 "None"))
  (for _array_element _outhits
    (if (or (== (.HitComponent (Collision|BreakHitResult _array_element)) Component) (== (.HitActor (Collision|BreakHitResult _array_element)) (LocalVariables|GetlOverlapedActor)))
      (LocalVariables|SetlNewLocation (.Location (Collision|BreakHitResult _array_element)))
      (if (> (CallFunction|CalcSummaryAbsorving) (Variables|Default|GetSpeedToDestroyPercent))
        (Game|SpawnActorfromClass "/Game/ProWeaponComponent/Blueprints/Actors/Projectiles/BP_PierceProjectile.BP_PierceProjectile_C" (Math|Transform|MakeTransform (LocalVariables|GetlNewLocation) (Transformation|GetActorRotation) "1,1,1") "AlwaysSpawn" (Components|GetOwner) (* (Variables|Default|GetDamage) (LocalVariables|GetlAbsorving)) (* (Variables|Default|GetSpeed) (LocalVariables|GetlAbsorving)) (Variables|Default|GetAccuracy) (Variables|Default|GetHitActors) 0 0)
        (return)
        (else
          (return)))))
  (LocalVariables|SetlNewLocation (+ (Transformation|GetActorLocation) (* (Transformation|GetActorForwardVector) 1e+01)))
  (if (> (CallFunction|CalcSummaryAbsorving) (Variables|Default|GetSpeedToDestroyPercent))
    (Game|SpawnActorfromClass "/Game/ProWeaponComponent/Blueprints/Actors/Projectiles/BP_PierceProjectile.BP_PierceProjectile_C" (Math|Transform|MakeTransform (LocalVariables|GetlNewLocation) (Transformation|GetActorRotation) "1,1,1") "AlwaysSpawn" (Components|GetOwner) (* (Variables|Default|GetDamage) (LocalVariables|GetlAbsorving)) (* (Variables|Default|GetSpeed) (LocalVariables|GetlAbsorving)) (Variables|Default|GetAccuracy) (Variables|Default|GetHitActors) 0 0)
    (return)
    (else
      (return))))