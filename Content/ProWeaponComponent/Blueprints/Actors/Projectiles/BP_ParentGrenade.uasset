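; Parent Blueprint for networked grenade projectiles that launch forward and explode after a timed fuse.
; BeginPlay adds a forward impulse to the skeletal mesh, then calls a server event that waits out the delay.
; The server multicasts the mesh location, applies radial damage slightly above it, and multicasts the explosion.
; The explosion multicast spawns particles and sound, hides the mesh, and destroys the actor shortly afterwards.
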(event Custom|BeginPlay%20%28%20SERVER%20%29
  (Utilities|FlowControl|Delay (Variables|Default|GetDelay))
  (CallFunction|SaveLocation(MULTICAST))
  (Rendering|SetVisibility (Variables|Default|GetSkeletalMesh) false false)
  (CallFunction|ProcessDamage)
  (CallFunction|Explosion(MULTICAST)))

(event Custom|Explosion%20%28%20MULTICAST%20%29
  (bind _skeletalmesh (Variables|Default|GetSkeletalMesh))
  (CallFunction|Explosion)
  (Utilities|IsValid _skeletalmesh
    (:Is%20Valid
      (Rendering|SetVisibility _skeletalmesh false false))
    (:Is%20Not%20Valid
      _))
  (Utilities|FlowControl|Delay 0.2)
  (Actor|DestroyActor))

(event Custom|SaveLocation%20%28%20MULTICAST%20%29
  (Variables|Default|SetLocation (Transformation|GetWorldLocation (Variables|Default|GetSkeletalMesh))))

(event EventBeginPlay
  (Physics|AddImpulse (Variables|Default|GetSkeletalMesh) (* (Transformation|GetActorForwardVector) (Variables|Default|GetImpulse)) "None" false)
  (CallFunction|BeginPlay(SERVER)))

(fn ConstructionScript)

(fn Explosion
  (Effects|SpawnEmitteratLocation "/Game/ProWeaponComponent/EpicContent/StarterContent/Particles/P_Explosion.P_Explosion" (Transformation|GetWorldLocation (Variables|Default|GetSkeletalMesh)) "0, 0, 0" "1.000000,1.000000,1.000000" false)
  (Audio|SpawnSoundatLocation "/Game/ProWeaponComponent/EpicContent/Audio/SN_Explosion.SN_Explosion" (Transformation|GetWorldLocation (Variables|Default|GetSkeletalMesh)) "0, 0, 0" 1.0 1.0 0.0 0 0 false)
  (return))

(fn ProcessDamage
  (Game|Damage|ApplyRadialDamage 1e+02 (+ (Variables|Default|GetLocation) "0, 0,30.000000") (Variables|Default|GetDamageRadius) 0 (Utilities|Array|MakeArray self) self 0 false "ECC_Visibility")
  (return))