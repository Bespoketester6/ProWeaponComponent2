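; Thrown C4 projectile for the ProWeaponComponent weapon system that turns into a placed charge when it lands.
; On hit, if it has speed, is not yet attached and struck something other than its owner, it aligns its up axis to the surface normal.
; It then spawns BP_C4_Attached at that transform, passing owner, damage and accuracy, and destroys itself.
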(event Collision|EventHit
  (params (MyComp :type Primitive%20Component%20Object%20Reference) (Other :type Actor%20Object%20Reference) (OtherComp :type Primitive%20Component%20Object%20Reference) (bSelfMoved :type Boolean) (HitLocation :type Vector :default "0, 0, 0") (HitNormal :type Vector :default "0, 0, 0") (NormalImpulse :type Vector :default "0, 0, 0") (Hit :type Hit%20Result%20Structure%20%28by%20ref%29))
  ;[0 0 0] Overwrite Event HIT
  (if (!= (Variables|Default|GetSpeed) 0.0)
    (if (and (not (Variables|Default|GetbAttached)) (!= Other (Components|GetOwner)))
      (Transformation|SetActorRotation (Math|Rotator|MakeRotfromZ HitNormal))
      (Game|SpawnActorfromClass "/Game/ProWeaponComponent/Blueprints/Actors/Special/BP_C4_Attached.BP_C4_Attached_C" (Transformation|GetActorTransform) "Undefined" (Components|GetOwner) (Variables|Default|GetDamage) (Variables|Default|GetAccuracy) 0)
      (Actor|DestroyActor))))

(fn ConstructionScript)