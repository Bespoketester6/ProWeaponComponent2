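; Timed grenade projectile that scales its blast sphere and explosion effect by Accuracy.
; BeginPlay starts delayed timers: visuals and sound run everywhere, while only the server damages actors overlapping the sphere.
; Server-side hits on non-owners run a damped Ricochet, whose true result triggers multicast destruction.
; An AttachC4 helper, not called here, traces along the mesh's down axis to attach to surfaces.
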(event EventBeginPlay
  ;[0 0 0] Begin Play
  (Utilities|FlowControl|Sequence
    (:then_0
      (Transformation|SetRelativeScale3D (Variables|Default|GetSphere) (* "5.000000,5.000000,5.000000" (Variables|Default|GetAccuracy)))
      (Utilities|Time|SetTimerbyFunctionName 0 "ExplosionVisual" (Variables|Default|GetExplosionDelay))
      (if (Networking|IsServer)
        (Utilities|Time|SetTimerbyFunctionName 0 "ExplosionCalcDamage" (Variables|Default|GetExplosionDelay))))))

(event Collision|EventHit
  (params (MyComp :type Primitive%20Component%20Object%20Reference) (Other :type Actor%20Object%20Reference) (OtherComp :type Primitive%20Component%20Object%20Reference) (bSelfMoved :type Boolean) (HitLocation :type Vector :default "0, 0, 0") (HitNormal :type Vector :default "0, 0, 0") (NormalImpulse :type Vector :default "0, 0, 0") (Hit :type Hit%20Result%20Structure%20%28by%20ref%29))
  ;[0 0 0] Overwrite Event HIT
  (if (Networking|IsServer)
    (if (not (== Other (Components|GetOwner)))
      (bind _success (CallFunction|Ricochet HitNormal 0.8 1e+02))
      (if _success
        (CallFunction|Destroy(MULTICAST))))))

(fn ConstructionScript)

(fn ExplosionVisual
  ;[0 0 0] Spawn Explosion Particle
  (Effects|SpawnEmitteratLocation "/Game/ProWeaponComponent/EpicContent/StarterContent/Particles/P_Explosion.P_Explosion" (+ (Transformation|GetActorLocation) (* (Math|Vector|GetUpVector (Variables|Default|GetSkeletalMesh)) 1e+01)) "0, 0, 0" (* "1.000000,1.000000,1.000000" (Variables|Default|GetAccuracy)))
  (Rendering|SetVisibility (Variables|Default|GetSkeletalMesh) false false)
  (Audio|SpawnSoundatLocation "/Game/ProWeaponComponent/EpicContent/ShooterGame/Sounds/Weapon_GrenadeLauncher/Mono/SN_GrenadeLauncher_Explosion03.SN_GrenadeLauncher_Explosion03" (Transformation|GetWorldLocation (Variables|Default|GetSkeletalMesh)) "0, 0, 0" 1.0 1.0 0.0 (CallFunction|GetSoundAttenuation) 0)
  (return))

(fn ExplosionCalcDamage
  ;[0 0 0] Calc Damage On Explose
  (for _array_element (Collision|GetOverlappingActors (Variables|Default|GetSphere) "/Script/Engine.Actor" :!class /Script/Engine.PrimitiveComponent)
    (Game|Damage|ApplyDamage _array_element (Variables|Default|GetDamage) 0 (Components|GetOwner)))
  (return))

(fn AttachC4
  (bind _returnvalue (Transformation|GetActorLocation))
  (bind _skeletalmesh (Variables|Default|GetSkeletalMesh))
  (bind _returnvalue_2 (Math|Vector|GetUpVector _skeletalmesh))
  ;[0 0 0] Attach C4 To Surface
  (bind _outhit (Collision|LineTraceByChannel (+ _returnvalue (* _returnvalue_2 1.0)) (+ _returnvalue (* _returnvalue_2 -1e+01)) "TraceTypeQuery1" false 0 "None"))
  (Utilities|IsValid (.HitComponent (Collision|BreakHitResult _outhit))
    (:Is%20Valid
      (Transformation|AttachComponentToComponent (.HitComponent (Collision|BreakHitResult _outhit)) "None" "KeepWorld" "KeepWorld" "KeepWorld" true)
      (Variables|Default|SetbAttached true)
      (return))
    (:Is%20Not%20Valid
      (return))))