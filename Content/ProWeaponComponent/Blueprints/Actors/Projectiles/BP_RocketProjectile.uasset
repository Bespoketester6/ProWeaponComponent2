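; Rocket projectile for the weapon component, a child projectile that explodes on impact.
; It overrides the parent's impact particle step to spawn an explosion emitter and sound at its location, then calls the parent version.
; ApplyDamage is overridden to deal radial damage around the projectile instead of to a single target.
; A multicast particle event repeats the same explosion effect and sound.
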(event EventParticle(MULTICAST)
  (params (Location :type Vector :default "0, 0, 0") (Rotation :type Rotator :default "0, 0, 0") (EmitterTemplate :type Particle%20System%20Object%20Reference) (Sound :type Sound%20Base%20Object%20Reference))
  ;[0 0 0] Particle
  (Effects|SpawnEmitteratLocation "/Game/ProWeaponComponent/EpicContent/StarterContent/Particles/P_Explosion.P_Explosion" (Transformation|GetActorLocation) (Transformation|GetActorRotation))
  (Audio|SpawnSoundatLocation "/Game/ProWeaponComponent/EpicContent/ShooterGame/Sounds/Weapon_GrenadeLauncher/Mono/SN_GrenadeLauncher_Explosion03.SN_GrenadeLauncher_Explosion03" (Transformation|GetActorLocation) "0, 0, 0" 1.0 1.0 0.0 "/Game/ProWeaponComponent/Assets/SoundSettings/SA_Realistic.SA_Realistic" 0))

(fn ConstructionScript
  (|CallParentFunction))

(fn SpawnImpactParicle
  (Effects|SpawnEmitteratLocation "/Game/ProWeaponComponent/EpicContent/StarterContent/Particles/P_Explosion.P_Explosion" (Transformation|GetActorLocation) (Transformation|GetActorRotation))
  (Audio|SpawnSoundatLocation "/Game/ProWeaponComponent/EpicContent/ShooterGame/Sounds/Weapon_GrenadeLauncher/Mono/SN_GrenadeLauncher_Explosion03.SN_GrenadeLauncher_Explosion03" (Transformation|GetActorLocation) "0, 0, 0" 1.0 1.0 0.0 "/Game/ProWeaponComponent/Assets/SoundSettings/SA_Realistic.SA_Realistic" 0)
  (bind _particle (|CallParentFunction))
  (return _particle 0))

(fn ApplyDamage
  (params (Target :type Actor%20Object%20Reference))
  ;[0 0 0] Radial Damage Apply
  (Game|Damage|ApplyRadialDamage (Variables|Default|GetDamage) (Transformation|GetActorLocation) 5e+02 0 0 self 0 false "ECC_Visibility")
  (return))