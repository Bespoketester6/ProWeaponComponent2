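; BP_ProjectileSpawner is a world actor that automatically fires projectiles at a fixed interval.
; On BeginPlay, only the server starts a looping timer at the Firerate interval that calls SpawnProjectile.
; Each call spawns a ParentProjectile at the Arrow component's world transform, owned by the spawner, passing in its Damage and Speed and a hard-coded accuracy.
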(event EventBeginPlay
  (if (Networking|IsServer)
    (Utilities|Time|SetTimerbyFunctionName 0 "SpawnProjectile" (Variables|Default|GetFirerate) true)))

(fn ConstructionScript)

(fn SpawnProjectile
  (Game|SpawnActorfromClass (Variables|Default|GetParentProjectile) (Transformation|GetWorldTransform (Variables|Default|GetArrow)) "Undefined" self (Variables|Default|GetDamage) (Variables|Default|GetSpeed) 2.0 0 0 0)
  (return))