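; BP_PlaceActor is a placement preview that shows whether an object can be placed at its current spot.
; It displays a configurable skeletal mesh and, on a looping timer, tints every material slot transparent green or red.
; Placement is valid when its owning BP_Weapon is closer than Params.BulletSpeed, which is repurposed as a range limit.
; The actor destroys itself once its Weapon reference becomes invalid.
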(event EventBeginPlay
  (Class|SkinnedMeshComponent|SetSkeletalMesh (Variables|Default|GetSkeletalMesh) (Variables|Default|GetMesh) true)
  (Utilities|Time|SetTimerbyFunctionName 0 "CanPlaceColor" 0.05 true))

(fn ConstructionScript)

(fn CanPlaceColor
  (Utilities|IsValid (Variables|Default|GetWeapon)
    (:Is%20Valid
      (if (CallFunction|CanPlace)
        (for _index (range 0 (Rendering|Material|GetNumMaterials (Variables|Default|GetSkeletalMesh)))
          (Rendering|Material|SetMaterial (Variables|Default|GetSkeletalMesh) _index "/Game/ProWeaponComponent/Assets/Materials/MI_GreenTransperent.MI_GreenTransperent"))
        (return)
        (else
          (for _index_2 (range 0 (Rendering|Material|GetNumMaterials (Variables|Default|GetSkeletalMesh)))
            (Rendering|Material|SetMaterial (Variables|Default|GetSkeletalMesh) _index_2 "/Game/ProWeaponComponent/Assets/Materials/MI_RedTransperent.MI_RedTransperent"))
          (return))))
    (:Is%20Not%20Valid
      (Actor|DestroyActor)
      (return))))

(fn CanPlace
  (bind _returnvalue (Components|GetOwner))
  (Utilities|IsValid _returnvalue
    (:Is%20Valid
      (bind _asbp_weapon (Utilities|Casting|CastToBP_Weapon _returnvalue)
        (:then
          (Utilities|IsValid _asbp_weapon
            (:Is%20Valid
              (return (< (Math|Vector|VectorLength (- (Transformation|GetActorLocation (Components|GetOwner)) (Transformation|GetActorLocation))) (.BulletSpeed (Utilities|Struct|BreakS_WeaponMainParams (Variables|/Game/ProWeaponComponent/Blueprints/Actors/BP_Weapon.BP_Weapon_C|GetParams _asbp_weapon))))))
            (:Is%20Not%20Valid
              (return false))))
        (:CastFailed
          (return false))))
    (:Is%20Not%20Valid
      (return false))))