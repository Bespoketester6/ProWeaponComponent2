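; An attached C4 charge that sticks to the surface beneath it and explodes after a delay.
; On BeginPlay a short trace along the mesh's down axis attaches the mesh to the hit component, then timers schedule the blast.
; Explosion emitter, sound and mesh hiding run on every instance where BeginPlay fires, while radial damage is scheduled only on the server.
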(event EventBeginPlay
  ;[0 0 0] Begin Play
  (CallFunction|AttachC4)
  (Utilities|Time|SetTimerbyFunctionName 0 "ExplosionVisual" (Variables|Default|GetExplosionDelay))
  (if (Networking|IsServer)
    (Utilities|Time|SetTimerbyFunctionName 0 "ExplosionCalcDamage" (Variables|Default|GetExplosionDelay))))

(fn ConstructionScript)

(fn ExplosionVisual
  ;[0 0 0] Explose Spawn Visual
  (Effects|SpawnEmitteratLocation "/Game/ProWeaponComponent/EpicContent/StarterContent/Particles/P_Explosion.P_Explosion" (+ (Transformation|GetActorLocation) (* (Math|Vector|GetUpVector (Variables|Default|GetSkeletalMesh)) 1e+01)) "0, 0, 0" (* "1.000000,1.000000,1.000000" (Variables|Float|GetAccuracy)))
  (Rendering|SetVisibility (Variables|Default|GetSkeletalMesh) false false)
  (Audio|SpawnSoundatLocation "/Game/ProWeaponComponent/EpicContent/ShooterGame/Sounds/Weapon_GrenadeLauncher/Mono/SN_GrenadeLauncher_Explosion03.SN_GrenadeLauncher_Explosion03" (Transformation|GetWorldLocation (Variables|Default|GetSkeletalMesh)) "0, 0, 0" 1.0 1.0 0.0 (CallFunction|GetSoundAttenuation) 0)
  (return))

(fn ExplosionCalcDamage
  ;[0 0 0] Calculate C4 Damage
  (Game|Damage|ApplyRadialDamage 1e+02 (Transformation|GetWorldLocation (Variables|Default|GetSkeletalMesh)) (Variables|Default|GetDamageRadius) 0 (Utilities|Array|MakeArray self) self 0 false "ECC_Visibility")
  (return))

(fn AttachC4
  (bind _returnvalue (Transformation|GetActorLocation))
  (bind _skeletalmesh (Variables|Default|GetSkeletalMesh))
  (bind _returnvalue_2 (Math|Vector|GetUpVector _skeletalmesh))
  ;[0 0 0] Attach C4
  (bind _outhit (Collision|LineTraceByChannel (+ _returnvalue (* _returnvalue_2 1.0)) (+ _returnvalue (* _returnvalue_2 -1e+01)) "TraceTypeQuery1" false 0 "None"))
  (Utilities|IsValid (.HitComponent (Collision|BreakHitResult _outhit))
    (:Is%20Valid
      (Transformation|AttachComponentToComponent (Variables|Default|GetSkeletalMesh) (.HitComponent (Collision|BreakHitResult _outhit)) "None" "KeepWorld" "KeepWorld" "KeepWorld" true)
      (Variables|Default|SetbAttached true)
      (return))
    (:Is%20Not%20Valid
      (return))))