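; Base grenade launcher weapon attachment that supplies its weapon data, ammo and muzzle location.
; On BeginPlay it loads its row from DT_AttachmentsWeapons, using WeaponAttachmentID as an index into the row names, attaches to its parent and passes the data to its owner.
; Getters expose the weapon data with current ammo and the Body's Muzzle socket location; the muzzle mesh getter reports failure.
; SetCurAmmo updates the stored ammo count.
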(event EventBeginPlay
  (CallFunction|ReadWeaponData)
  (CallFunction|ReadData)
  (CallFunction|AttachtoParent)
  (Utilities|IsValid (Components|GetOwner)
    (:Is%20Valid
      (Class|ABPISetAdditionalData|SetAdditionalData(Message) (Components|GetOwner) (Variables|Params|GetWeaponData)))
    (:Is%20Not%20Valid
      (CallFunction|PrintError "Parent doesn't init in Grenade Laucnher"))))

(event EventSetCurAmmo
  (params (Ammo :type Integer))
  (Variables|Params|SetCurAmmo Ammo))

(fn ConstructionScript
  (|CallParentFunction))

(fn ReadWeaponData
  ;[0 0 0] Read Weapon Data From Attachments Weapons Datatable
  (bind _outrownames (DataTable|GetDataTableRowNames "/Game/ProWeaponComponent/Blueprints/Datatables/Attachments/DT_AttachmentsWeapons.DT_AttachmentsWeapons"))
  (bind _returnvalue (Utilities|GetDataTableRow "/Game/ProWeaponComponent/Blueprints/Datatables/Attachments/DT_AttachmentsWeapons.DT_AttachmentsWeapons" (Utilities|Array|Get(acopy) _outrownames (Variables|Settings|GetWeaponAttachmentID)))
    (:then
      (Variables|Params|SetWeaponData _returnvalue)
      (return))
    (:RowNotFound
      (return))))

(fn GetMuzzleLocation
  (return true (Transformation|GetSocketLocation (Variables|Default|GetBody) "Muzzle")))

(fn GetMuzzleMesh
  (return false 0))

(fn GetWeaponData
  (return true (Variables|Params|GetWeaponData) (Variables|Params|GetCurAmmo)))