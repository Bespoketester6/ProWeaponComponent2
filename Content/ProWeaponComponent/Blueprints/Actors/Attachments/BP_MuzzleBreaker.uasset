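; BP_MuzzleBreaker is a muzzle brake weapon attachment that halves recoil and scales down the accuracy and damage values.
; It answers attachment queries with a Success flag and a value, covering those scales, a replacement assault rifle fire sound and its own mesh as the muzzle mesh.
; The muzzle location comes from the Muzzle socket on that mesh, and the event graph holds no logic.
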(event EventBeginPlay)

(event Collision|EventActorBeginOverlap
  (params (OtherActor :type Actor%20Object%20Reference)))

(event EventTick
  (params (DeltaSeconds :type Float%20%28single-precision%29)))

(fn ConstructionScript
  (|CallParentFunction))

(fn GetAccuracyScale
  (return true 0.8))

(fn GetDamageScale
  (return true 0.9))

(fn GetFireSound
  (params (DefaultSound :type Sound%20Base%20Object%20Reference))
  (return true "/Game/ProWeaponComponent/EpicContent/ShooterGame/Sounds/Weapon_AssaultRifle/Mono/SN_AssaultRifle_Shot.SN_AssaultRifle_Shot"))

(fn GetMuzzleLocation
  (return true (Transformation|GetSocketLocation (Variables|Default|GetMesh) "Muzzle")))

(fn GetMuzzleMesh
  (return true (Variables|Default|GetMesh)))

(fn GetRecoilScale
  (return true 0.5))