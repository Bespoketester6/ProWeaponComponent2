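; Parent weapon laser sight attachment that shows where the weapon aims, with toggleable dot and click sound.
; Roguelike and Platformer modes spawn a beam particle and mouse-follow target actor; Tick points the beam at the owning character's look-at location.
; Without a beam, Tick places the dot there, or at a forward muzzle trace while sprinting, reloading or swapping weapons.
; The dot scales with distance from the player pawn.
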(event EventAttachmentEventA
  ;[0 0 0] Turn Laser Sight On/Off
  (Variables|Default|SetbTurnOn (not (Variables|Default|GetbTurnOn)))
  (Development|SetHiddeninGame (Variables|Default|GetDot) (not (Variables|Default|GetbTurnOn)) false)
  (CallFunction|PlaySound(MULTICAST) "/Game/ProWeaponComponent/Assets/Sounds/Weapons/Attachments/SN_ButtonPress.SN_ButtonPress"))

(event EventBeginPlay
  ;[0 0 0] Overwrite BeginPlay
  (CallFunction|ReadData)
  (CallFunction|AttachtoParent)
  ;[0 0 0] Platformer And Roguelike Use Particle For Laserbeam
  (bind _buse (Class|BPIWCCharacter|GetCharacterMode(Message) (Components|GetOwner (Components|GetOwner))))
  (switch Utilities|FlowControl|Switch|SwitchonE_CharacterMode _buse
    (:NewEnumerator2
      _)
    (:NewEnumerator3
      _))
  (bind _returnvalue (Effects|SpawnEmitterAttached "/Game/ProWeaponComponent/Assets/Particle/P_LaserBeam.P_LaserBeam" (Variables|Default|GetBody) "LaserOut"))
  (bind _output_get (Variables|Default|SetBeam _returnvalue))
  (bind _returnvalue_2 (Game|SpawnActorfromClass "/Game/ProWeaponComponent/Blueprints/Actors/BP_ActorFollowMouse.BP_ActorFollowMouse_C" (Math|Transform|MakeTransform "0, 0, 0" "0, 0, 0" "1,1,1") "Undefined" self 0))
  (Utilities|IsValid _output_get
    (:Is%20Valid
      (Effects|Components|ParticleSystem|SetActorParameter _output_get "Target" _returnvalue_2))))

(event EventTick
  (params (DeltaSeconds :type Float%20%28single-precision%29))
  ;[0 0 0] For FPS & TPS interpolate laser sight dot position
  (Utilities|IsValid (Variables|Default|GetBeam)
    (:Is%20Valid
      (bind _location (Class|BPIWCCharacter|GetLookatLocation(Message) (Components|GetOwner (Components|GetOwner)) 0.0))
      (Class|ParticleSystemComponent|SetBeamTargetPoint (Variables|Default|GetBeam) 0 _location))
    (:Is%20Not%20Valid
      (bind _location_2 (Class|BPIWCCharacter|GetLookatLocation(Message) (Components|GetOwner (Components|GetOwner)) 0.0))
      (Transformation|SetWorldLocation (Variables|Default|GetDot) (select (CallFunction|BShouldDraw) _location_2 (CallFunction|GetForwardLocation)) false true)
      (Transformation|SetWorldScale3D (Variables|Default|GetDot) (* (* "0.001000,0.001000,0.001000" (/ (Math|Vector|VectorLength (- (Transformation|GetWorldLocation (Variables|Default|GetDot)) (Transformation|GetActorLocation (Game|Player|GetPlayerPawn 0)))) 3e+02)) 6.0)))))

(fn ConstructionScript
  (|CallParentFunction))

(fn BShouldDraw
  (bind _bsprint (Class|BPIWCCharacter|GetSprint(Message) (Components|GetOwner (Components|GetOwner))))
  (if _bsprint
    (return false)
    (else
      (bind _asbp_weapon (Utilities|Casting|CastToBP_Weapon (Components|GetOwner))
        (:then
          (if (Variables|/Game/ProWeaponComponent/Blueprints/Actors/BP_Weapon.BP_Weapon_C|GetbInReload _asbp_weapon)
            (return false)
            (else
              (bind _weaponcomponent (Class|BPIGetWeaponComponent|GetWeaponComponent(Message) (Components|GetOwner (Components|GetOwner))))
              (if (Variables|/Game/ProWeaponComponent/Blueprints/Components/BPC_WeaponComponent.BPC_WeaponComponent_C|GetbSwapWeapons _weaponcomponent)
                (return false)
                (else
                  (return true))))))
        (:CastFailed
          (return false))))))

(fn GetForwardLocation
  (bind _returnvalue (Transformation|GetActorForwardVector))
  (bind _body (Variables|Default|GetBody))
  (bind _returnvalue_2 (Transformation|GetSocketLocation _body "LaserOut"))
  (bind _returnvalue_3 (* _returnvalue 1e+05))
  (bind _returnvalue_4 (+ _returnvalue_3 "0, 0, 0"))
  (bind _returnvalue_5 (+ _returnvalue_2 _returnvalue_4))
  (bind (_outhit _returnvalue_6) (Collision|LineTraceByChannel _returnvalue_2 _returnvalue_5 "TraceTypeQuery1" false 0 "None"))
  (if _returnvalue_6
    (return (.Location (Collision|BreakHitResult _outhit)))
    (else
      (return _returnvalue_5))))