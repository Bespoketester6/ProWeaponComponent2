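; BP_ParentSight is a weapon sight attachment Blueprint with a switchable reticle dot.
; On BeginPlay it reads its data, attaches to its parent and applies the current dot material to a plane.
; Attachment event B cycles through the dot materials with wraparound and multicasts a button-press sound.
; It supplies aim-down-sights camera and hand offsets selected by weapon ID, so alignment varies per weapon.
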(event EventBeginPlay
  ;[0 0 0] Overwrite
  (CallFunction|ReadData)
  (CallFunction|AttachtoParent)
  ;[0 0 0] Set Dot From Array
  (Rendering|Material|SetMaterial (Variables|Default|GetPlane) 0 (Utilities|Array|Get(acopy) (Variables|Default|GetMaterials) (Variables|Default|GetCurDot))))

(event EventAttachmentEventB
  ;[0 0 0] Change Sight Dot
  (Variables|Default|SetCurDot (Math|Integer|%(Integer) (+ (Variables|Default|GetCurDot) 1) (Utilities|Array|Length (Variables|Default|GetMaterials))))
  (Rendering|Material|SetMaterial (Variables|Default|GetPlane) 0 (Utilities|Array|Get(acopy) (Variables|Default|GetMaterials) (Variables|Default|GetCurDot)))
  (CallFunction|PlaySound(MULTICAST) "/Game/ProWeaponComponent/Assets/Sounds/Weapons/Attachments/SN_ButtonPress.SN_ButtonPress"))

(fn ConstructionScript
  (|CallParentFunction))

(fn GetAimCameraOffset
  (return true (Utilities|Select :Index (Variables|Default|GetWeaponID) :Option%200 "0, 0, 0" :Option%201 "0,-0.130000,-0.970000" :Option%202 "0,0.050000,0.930000" :Option%203 "0,-0.050000,1.960000" :Option%204 "0, 0, 0")))

(fn GetAimHandsOffset
  (return true (Utilities|Select :Index (Variables|Default|GetWeaponID) :Option%200 "0, 0, 0" :Option%201 "0,0.150000,-0.500000" :Option%202 "0,0.100000,-1.200000" :Option%203 "-10.000000,0.100000,-2.100000" :Option%204 "0, 0, 0")))