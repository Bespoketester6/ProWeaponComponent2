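; Base silencer attachment Blueprint for the weapon component system, modifying how a weapon fires.
; It answers attachment queries with a success flag plus fixed multipliers that reduce damage and recoil.
; A lookup map swaps the default rifle or pistol shot sound for its silenced version.
; It also supplies its own mesh and that mesh's Muzzle socket as the firing muzzle.
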(event EventBeginPlay)

(event Collision|EventActorBeginOverlap
  (params (OtherActor :type Actor%20Object%20Reference)))

(event EventTick
  (params (DeltaSeconds :type Float%20%28single-precision%29)))

(fn ConstructionScript
  (|CallParentFunction))

(fn GetDamageScale
  (return true 0.8))

(fn GetFireSound
  (params (DefaultSound :type Sound%20Base%20Object%20Reference))
  (return true (.Value (Utilities|Map|Find (Utilities|Map|MakeMap "/Game/ProWeaponComponent/Assets/Sounds/Weapons/Rifle/SN_Rifle_Shot.SN_Rifle_Shot" "/Game/ProWeaponComponent/Assets/Sounds/Weapons/Rifle/SN_Silenced_Rifle_Shot.SN_Silenced_Rifle_Shot" "/Game/ProWeaponComponent/Assets/Sounds/Weapons/Pistol/SN_Pistol_Shot.SN_Pistol_Shot" "/Game/ProWeaponComponent/Assets/Sounds/Weapons/Pistol/SN_Silenced_Pistol_Shot.SN_Silenced_Pistol_Shot") DefaultSound))))

(fn GetMuzzleLocation
  (return true (Transformation|GetSocketLocation (Variables|Default|GetMesh) "Muzzle")))

(fn GetMuzzleMesh
  (return true (Variables|Default|GetMesh)))

(fn GetRecoilScale
  (return true 0.5))