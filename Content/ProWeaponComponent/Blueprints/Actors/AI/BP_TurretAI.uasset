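; AI turret that automatically turns toward and fires on Characters entering its detection sphere.
; The latest overlapping Character becomes the target, cleared when that one leaves.
; Server BeginPlay starts fast looping timers that interpolate rotation toward the target and pulse the weapon component's UseWeapon while the target is alive.
; GetLookAtLocation is overridden to aim at the target's center height, or straight ahead without a target.
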(event OnComponentBeginOverlap(Sphere)
  (params (OverlappedComponent :type Primitive%20Component%20Object%20Reference) (OtherActor :type Actor%20Object%20Reference) (OtherComp :type Primitive%20Component%20Object%20Reference) (OtherBodyIndex :type Integer) (bFromSweep :type Boolean) (SweepResult :type Hit%20Result%20Structure%20%28by%20ref%29))
  ;[0 0 0] 1. INIT TARGET ACTOR
  (if (!= OtherActor self)
    (bind _ascharacter (Utilities|Casting|CastToCharacter OtherActor))
    (Variables|Default|SetTargetActor _ascharacter)))

(event OnComponentEndOverlap(Sphere)
  (params (OverlappedComponent :type Primitive%20Component%20Object%20Reference) (OtherActor :type Actor%20Object%20Reference) (OtherComp :type Primitive%20Component%20Object%20Reference) (OtherBodyIndex :type Integer))
  ;[0 0 0] 1. INIT TARGET ACTOR
  (if (== OtherActor (Variables|Default|GetTargetActor))
    (Variables|Default|SetTargetActor 0)))

(event Custom|BeginPlay%20%28%20SERVER%20%29
  ;[0 0 0] 3. INIT FIRE LOGIC
  (Utilities|Time|SetTimerbyEvent (delegate Custom|FireEvent) 0.01 true)
  (Utilities|Time|SetTimerbyEvent (delegate Custom|RotateToTarget) 0.01 true))

(event Custom|FireEvent
  ;[0 0 0] 3. INIT FIRE LOGIC
  (Utilities|IsValid (Variables|Default|GetTargetActor)
    (:Is%20Valid
      (bind _balive (Class|BPIWCCharacter|GetIsAlive(Message) (Variables|Default|GetTargetActor)))
      (if _balive
        (Default|UseWeapon (Variables|Default|GetBPC_WeaponComponent) true)
        (Default|UseWeapon (Variables|Default|GetBPC_WeaponComponent) false)))))

(event Custom|RotateToTarget
  ;[0 0 0] 3. INIT FIRE LOGIC
  (Utilities|IsValid (Variables|Default|GetTargetActor)
    (:Is%20Valid
      (Transformation|SetActorRotation (Math|Interpolation|RInterpTo (Transformation|GetActorRotation) (Math|Rotator|FindLookatRotation (Transformation|GetActorLocation) (Transformation|GetActorLocation (Variables|Default|GetTargetActor))) (Utilities|Time|GetWorldDeltaSeconds) 25.0)))))

(event EventBeginPlay
  ;[0 0 0] 3. INIT FIRE LOGIC
  (|CallParentFunction)
  (CallFunction|BeginPlay(SERVER)))

(fn ConstructionScript
  (|CallParentFunction))

(fn GetLookatLocation
  (params (Accuracy :type Float%20%28single-precision%29))
  (bind _targetactor (Variables|Default|GetTargetActor))
  (Utilities|IsValid (Variables|Default|GetTargetActor)
    (:Is%20Valid
      (bind _height (Class|BPIGetActorCenterLocation|GetActorCenterHeight(Message) _targetactor))
      (return (+ (Math|Vector|MakeVector 0.0 0.0 _height) (Transformation|GetActorLocation _targetactor)) "0, 0, 0"))
    (:Is%20Not%20Valid
      (return (+ (* (Transformation|GetActorForwardVector) 1e+03) (Transformation|GetActorLocation)) "0, 0, 0"))))