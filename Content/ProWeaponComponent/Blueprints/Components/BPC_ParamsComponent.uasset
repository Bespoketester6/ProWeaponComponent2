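; Actor component that manages a character's health, stamina, death and respawn.
; A looping server timer regenerates both stats, drains stamina during sprint and stops sprinting when empty, though health regen uses HealthStartRegenDelay as rate and MaxStamina as cap.
; Lethal damage multicasts pelvis-down ragdoll and an optional local respawn menu.
; Respawn resets stats, reattaches the mesh and teleports the owner to a random PlayerStart.
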(event Custom|BeginPlay%20%28%20SERVER%20%29
  ;[0 0 0] Server Event
  (Utilities|Time|SetTimerbyFunctionName 0 "ParamsRegeneration" 0.1 true))

(event Custom|EnableRagdoll%20%28%20MULTICAST%20%29
  ;[0 0 0] Ragdoll
  (Damage|EnableRagdoll))

(event Custom|Respawn%20%28%20SERVER%20%29
  ;[0 0 0] Respawn
  (Variables|Boolean|SetbDead false)
  (Variables|Params|SetCurHealth 1e+02)
  (Variables|Params|SetCurStamina 1e+02)
  (Variables|Boolean|SetbAllowToRegenHealth true)
  (Variables|Boolean|SetbAllowToRegenStamina true)
  (CallFunction|DisableRagdoll(MULTICAST)))

(event Custom|SpawnRespawnMenu%20%28%20MULTICAST%20%29
  ;[0 0 0] Spawn Respawn Menu
  (if (== (Game|Player|GetPlayerPawn 0) (Components|GetOwner))
    (bind _returnvalue (UserInterface|CreateWidget "/Game/ProWeaponComponent/Blueprints/Widget/Main/W_RespawnMenu.W_RespawnMenu_C" (Game|GetPlayerController 0)))
    (Utilities|IsValid _returnvalue
      (:Is%20Valid
        (UserInterface|Viewport|AddtoViewport _returnvalue 0)
        (Variables|/Script/Engine.PlayerController|SetbShowMouseCursor (Game|GetPlayerController 0) true)))))

(event Custom|DisableRagdoll%20%20%28%20MULTICAST%20%29
  ;[0 0 0] Ragdoll
  (Damage|DisableRagdoll))

(event EventBeginPlay
  ;[0 0 0] Default
  (CallFunction|BeginPlay(SERVER)))

(fn ApplyDamage
  (params (Damage :type Float%20%28single-precision%29))
  (bind _output_get (Variables|Params|SetCurHealth (Math|Float|Max(Float) (+ (* Damage -1.0) (Variables|Params|GetCurHealth)) 0.0)))
  (if (<= _output_get 0.0)
    (if (not (Variables|Boolean|GetbDead))
      (Variables|Boolean|SetbDead true)
      (Damage|DeadEvent)
      (Variables|Boolean|SetbAllowToRegenHealth false)
      (return))
    (elif (!= (Variables|Settings|GetHealthStartRegenDelay) 0.0)
      (Variables|Boolean|SetbAllowToRegenHealth false)
      (if (== (Variables|Settings|GetHealthStartRegenDelay) -1.0)
        (return)
        (else
          (Utilities|Time|SetTimerbyFunctionName 0 "AllowToRegenHealth" (Variables|Settings|GetHealthStartRegenDelay))
          (return)))
      (else
        (return)))))

(fn DeadEvent
  (CallFunction|EnableRagdoll(MULTICAST))
  (if (Variables|Settings|GetbShouldSpawnRespawnMenu)
    (CallFunction|SpawnRespawnMenu(MULTICAST))
    (return)
    (else
      (return))))

(fn EnableRagdoll
  (bind _ascharacter (Utilities|Casting|CastToCharacter (Components|GetOwner))
    (:then
      (Collision|SetCollisionEnabled (Variables|/Script/Engine.Character|GetCapsuleComponent _ascharacter) "NoCollision")
      (bind _skeletalmesh (Class|BPIWCCharacter|GetClientMesh(Message) (Components|GetOwner)))
      (bind _output_get (LocalVariables|SetlSkMesh _skeletalmesh))
      (Variables|Transform|SetAttachParent (Transformation|GetAttachParent (LocalVariables|GetlSkMesh)))
      (Variables|Transform|SetMeshRelativeTransform (Transformation|GetRelativeTransform _output_get))
      (Collision|SetCollisionObjectType _output_get "ECC_PhysicsBody")
      (Collision|SetCollisionEnabled _output_get "QueryAndPhysics")
      (Collision|SetCollisionResponsetoChannel _output_get "ECC_GameTraceChannel1" "ECR_Ignore")
      (Class|SkeletalMeshComponent|SetAllBodiesBelowSimulatePhysics _output_get (Utilities|Name|MakeLiteralName "pelvis") true true)
      (Animation|Montage|MontageStop (Components|SkeletalMesh|GetAnimInstance (LocalVariables|GetlSkMesh)) 0.2 0)
      (return))
    (:CastFailed
      (return))))

(fn ParamsRegeneration
  ;[0 0 0] Force Events
  (Tick|CheckForceEvents)
  ;[0 0 0] Regen Stamina
  (Variables|Params|SetCurStamina (Math|Float|Max(Float) (Math|Float|Min(Float) (Variables|Params|GetMaxStamina) (+ (Variables|Params|GetCurStamina) (select (Boolean|ShouldRemoveStamina) -1.5 (select (Variables|Boolean|GetbAllowToRegenStamina) (/ (Variables|Settings|GetStaminaRegenPerSec) 1e+01) 0.0)))) 0.0))
  ;[0 0 0] Regen Health
  (Variables|Params|SetCurHealth (Math|Float|Min(Float) (Variables|Params|GetMaxStamina) (+ (Variables|Params|GetCurHealth) (select (Variables|Boolean|GetbAllowToRegenHealth) (/ (Variables|Settings|GetHealthStartRegenDelay) 1e+01) 0.0))))
  (return))

(fn AllowtoRegenHealth
  (Variables|Boolean|SetbAllowToRegenHealth true)
  (return))

(fn AllowtoRegenStamina
  (Variables|Boolean|SetbAllowToRegenStamina true)
  (return))

(fn ShouldRemoveStamina
  (bind _bsprint (Class|BPIWCCharacter|GetSprint(Message) (Components|GetOwner)))
  (if _bsprint
    (if (!= (Variables|Settings|GetStaminaStartRegenDelay) 0.0)
      (Variables|Boolean|SetbAllowToRegenStamina false)
      (if (== (Variables|Settings|GetStaminaStartRegenDelay) -1.0)
        (return false)
        (else
          (Utilities|Time|SetTimerbyFunctionName 0 "AllowToRegenStamina" (Variables|Settings|GetStaminaStartRegenDelay))
          (return true)))
      (else
        (return true)))
    (else
      (return false))))

(fn RemoveStaminaifCan
  (params (ToRemove :type Float%20%28single-precision%29))
  (if (>= (Variables|Params|GetCurStamina) ToRemove)
    (Variables|Params|SetCurStamina (- (Variables|Params|GetCurStamina) ToRemove))
    (return true)
    (else
      (return false))))

(fn CheckForceEvents
  ;[0 0 0] If don't have Stamina Stop Sprinting
  (if (< (Variables|Params|GetCurStamina) 1.0)
    (bind _bsprint (Class|BPIWCCharacter|GetSprint(Message) (Components|GetOwner)))
    (if _bsprint
      (Class|BPIWCCharacter|StopSprint(Message) (Components|GetOwner))
      (return)
      (else
        (return)))
    (else
      (return))))

(fn DisableRagdoll
  (bind _ascharacter (Utilities|Casting|CastToCharacter (Components|GetOwner))
    (:then
      (Collision|SetCollisionEnabled (Variables|/Script/Engine.Character|GetCapsuleComponent _ascharacter) "QueryAndPhysics")
      (bind _skeletalmesh (Class|BPIWCCharacter|GetClientMesh(Message) (Components|GetOwner)))
      (bind _output_get (LocalVariables|SetlSkMesh _skeletalmesh))
      (Collision|SetCollisionObjectType _output_get "ECC_GameTraceChannel3")
      (Collision|SetCollisionEnabled _output_get "QueryAndPhysics")
      (Collision|SetCollisionResponsetoChannel _output_get "ECC_GameTraceChannel1" "ECR_Block")
      (Class|SkeletalMeshComponent|SetAllBodiesBelowSimulatePhysics _output_get (Utilities|Name|MakeLiteralName "pelvis") false true)
      (Transformation|AttachComponentToComponent (LocalVariables|GetlSkMesh) (Variables|Transform|GetAttachParent) "None" "KeepRelative" "KeepRelative" "KeepRelative" true)
      (Transformation|SetRelativeTransform (LocalVariables|GetlSkMesh) (Variables|Transform|GetMeshRelativeTransform) false true)
      (Animation|Montage|MontageStop (Components|SkeletalMesh|GetAnimInstance (LocalVariables|GetlSkMesh)) 0.2 0)
      (bind _outactors (Actor|GetAllActorsOfClass "/Script/Engine.PlayerStart"))
      (Transformation|SetActorLocation (Components|GetOwner) (Transformation|GetActorLocation (Utilities|Array|Get(acopy) _outactors (Math|Random|RandomInteger (Utilities|Array|Length _outactors)))) false true)
      (return))
    (:CastFailed
      (return))))