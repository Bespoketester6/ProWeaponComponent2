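; Blueprint function library of shared static helpers for the weapon component system, covering impact effects, input and locomotion checks, and lookups.
; Hard-coded maps turn physical materials into impact particles and sounds, and the weapons table defaults to DT_Weapons unless a BP_CustomDatatable actor exists.
; Visibility traces find the actor ahead within range and check headroom before standing or crouching.
; Pawn and HUD state are read through message calls.
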(fn PhysicMaterialtoParticle
  (params (Class :type Physical%20Material%20Object%20Reference))
  (return (.Value (Utilities|Map|Find (Utilities|Map|MakeMap "/Game/ProWeaponComponent/Blueprints/PhysicMaterials/PM_Default.PM_Default" "/Game/ProWeaponComponent/EpicContent/ShooterGame/Effects/ParticleSystems/Weapons/AssaultRifle/Impacts/P_AssaultRifle_IH.P_AssaultRifle_IH" "/Game/ProWeaponComponent/Blueprints/PhysicMaterials/PM_Character.PM_Character" "/Game/ProWeaponComponent/EpicContent/ShooterGame/Effects/ParticleSystems/Gameplay/Player/P_body_bullet_impact.P_body_bullet_impact" "/Game/ProWeaponComponent/Blueprints/PhysicMaterials/PM_Character_Crit.PM_Character_Crit" "/Game/ProWeaponComponent/EpicContent/ShooterGame/Effects/ParticleSystems/Gameplay/Player/P_body_bullet_impact.P_body_bullet_impact") Class))))

(fn PrintError
  (params (InText :type Text))
  (Development|PrintText 0 (Utilities|Text|FormatText "Error: {0}" InText) true true "(R=1.000000,G=0.000000,B=0.000000,A=1.000000)" 4.0)
  (return))

(fn IsOwnerClient
  (params (Owner :type Actor%20Object%20Reference))
  (if (== Owner (Game|Player|GetPlayerPawn 0))
    (if (Networking|IsDedicatedServer)
      (return false)
      (else
        (return true)))
    (else
      (return false))))

(fn InputEnabled
  (bind _true (Class|BPIWCHUD|IsinHUD(Message) (CallFunction|GetWCHUD)))
  (if (not _true)
    (bind _balive (Class|BPIWCCharacter|GetIsAlive(Message) (Game|Player|GetPlayerPawn 0)))
    (if _balive
      (return true)
      (else
        (return false)))
    (else
      (return false))))

(fn GetWCHUD
  (bind _returnvalue (Game|GetPlayerController 0))
  (Utilities|IsValid _returnvalue
    (:Is%20Valid
      (return (HUD|GetHUD _returnvalue)))
    (:Is%20Not%20Valid
      (return 0))))

(fn GetRandomMontagefromArray
  (params (Array :type Array%20of%20Anim%20Montage%20Object%20References))
  (if (== (Utilities|Array|Length Array) 0)
    (return 0)
    (else
      (return (Utilities|Array|Get(acopy) Array (Math|Random|RandomInteger (Utilities|Array|Length Array)))))))

(fn PhysicMaterialtoImpactSound
  (params (PhysicMaterial :type Physical%20Material%20Object%20Reference))
  (return (.Value (Utilities|Map|Find (Utilities|Map|MakeMap "/Game/ProWeaponComponent/Blueprints/PhysicMaterials/PM_Character_Crit.PM_Character_Crit" "/Game/ProWeaponComponent/Assets/Sounds/Impacts/SN_BodyImpact.SN_BodyImpact" "/Game/ProWeaponComponent/Blueprints/PhysicMaterials/PM_Character.PM_Character" "/Game/ProWeaponComponent/Assets/Sounds/Impacts/SN_BodyImpact.SN_BodyImpact" "/Game/ProWeaponComponent/Blueprints/PhysicMaterials/PM_Default.PM_Default" "/Game/ProWeaponComponent/Assets/Sounds/Impacts/SN_WallImpact.SN_WallImpact") PhysicMaterial))))

(fn GetForwardActor
  (params (Target :type Actor%20Object%20Reference) (DistanceLimit :type Float%20%28single-precision%29))
  (bind _location (Class|BPIWCCharacter|GetLookatLocation(Message) Target 0.0))
  (bind (_outhit _returnvalue) (Collision|LineTraceByChannel 0 (Transformation|GetActorLocation Target) _location "TraceTypeQuery1" false (Utilities|Array|MakeArray Target) "None"))
  (if _returnvalue
    (if (<= (.Distance (Collision|BreakHitResult _outhit)) DistanceLimit)
      (return (.HitActor (Collision|BreakHitResult _outhit)))
      (else
        (return 0)))
    (else
      (return 0))))

(fn GetUsingWeaponsDatatable
  (bind _returnvalue (Actor|GetActorOfClass 0 "/Game/ProWeaponComponent/Blueprints/Actors/BP_CustomDatatable.BP_CustomDatatable_C"))
  (Utilities|IsValid _returnvalue
    (:Is%20Valid
      (bind _datatable (Default|GetDatatable _returnvalue))
      (return _datatable))
    (:Is%20Not%20Valid
      (return "/Game/ProWeaponComponent/Blueprints/Datatables/Main/DT_Weapons.DT_Weapons"))))

(fn CanChangeLocomotion
  (params (Pawn :type Pawn%20Object%20Reference) (Locomotion :type E_LocomotionType%20Enum :default "NewEnumerator0"))
  (bind _changelocomotion (Class|BPIWCCharacter|GetChangeLocomotion(Message) Pawn))
  (if _changelocomotion
    (return false)
    (else
      (switch Utilities|FlowControl|Switch|SwitchonE_LocomotionType Locomotion
        (:NewEnumerator0
          _)
        (:NewEnumerator1
          _)
        (:NewEnumerator2
          (return true)))
      (LocalVariables|SetlPawnLocation (Transformation|GetActorLocation Pawn))
      (bind _returnvalue (Collision|LineTraceByChannel 0 (LocalVariables|GetlPawnLocation) (+ (LocalVariables|GetlPawnLocation) (Utilities|Select :Index Locomotion :NewEnumerator0 "0, 0,130.000000" :NewEnumerator1 "0.000000,0.000000,75.000000" :NewEnumerator2 "0, 0, 0")) "TraceTypeQuery1" false (Utilities|Array|MakeArray Pawn) "None"))
      (if (not _returnvalue)
        (return true)
        (else
          (return false))))))