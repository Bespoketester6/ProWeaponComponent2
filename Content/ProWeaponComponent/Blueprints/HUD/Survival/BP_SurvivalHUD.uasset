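; BP_SurvivalHUD creates the W_SurvivalHUD widget on BeginPlay, adds it to the viewport, and serves as the control point for the survival HUD.
; SwapShowAttachmentsMenu toggles the attachments panel, the mouse cursor, and the input mode between Game and UI and Game Only.
; Update and UpdateWeapons forward refreshes to the widget and its weapons panel, while IsInHUD reports whether the attachments menu is open.
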(event EventBeginPlay
  (bind _returnvalue (UserInterface|CreateWidget "/Game/ProWeaponComponent/Blueprints/HUD/Survival/W_SurvivalHUD.W_SurvivalHUD_C" (Game|GetPlayerController 0)))
  (bind _output_get (Variables|Default|SetHUD _returnvalue))
  (UserInterface|Viewport|AddtoViewport _output_get 0))

(event EventSwapShowAttachmentsMenu
  (bind _returnvalue (Game|GetPlayerController 0))
  (bind _hud (Variables|Default|GetHUD))
  (bind _w_attachmentspanel (Variables|/Game/ProWeaponComponent/Blueprints/HUD/Survival/W_SurvivalHUD.W_SurvivalHUD_C|GetW_AttachmentsPanel _hud))
  (Variables|Boolean|SetAttachmentsShowed (not (Variables|Boolean|GetAttachmentsShowed)))
  (Widget|SetVisibility _w_attachmentspanel (select (Variables|Boolean|GetAttachmentsShowed) "Visible" "Hidden"))
  (Variables|/Script/Engine.PlayerController|SetbShowMouseCursor _returnvalue (Variables|Boolean|GetAttachmentsShowed))
  (if (Variables|Boolean|GetAttachmentsShowed)
    (Input|SetInputModeGameandUI _returnvalue _w_attachmentspanel "DoNotLock" true)
    (else
      (Input|SetInputModeGameOnly _returnvalue))))

(event EventUpdate
  (Default|Update (Variables|Default|GetHUD)))

(event EventUpdateWeapons
  (Default|Update (Variables|/Game/ProWeaponComponent/Blueprints/HUD/Survival/W_SurvivalHUD.W_SurvivalHUD_C|GetW_WeaponsPanel (Variables|Default|GetHUD))))

(fn ConstructionScript)

(fn IsinHUD
  (return (Variables|Boolean|GetAttachmentsShowed)))