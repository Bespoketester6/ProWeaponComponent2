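; BP_CompetitiveHUD is the HUD manager for the competitive mode, creating the W_CompetitiveHUD widget on BeginPlay and adding it to the viewport.
; Events toggle the attachments panel and the CS:GO-style weapon shop, and forward refresh calls to the whole HUD or just the weapon panel.
; FocusHUD switches cursor and input mode between Game-and-UI and game-only depending on open menus, which IsInHUD also reports.
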(event EventBeginPlay
  (bind _returnvalue (UserInterface|CreateWidget "/Game/ProWeaponComponent/Blueprints/HUD/Competitive/W_CompetitiveHUD.W_CompetitiveHUD_C" (Game|GetPlayerController 0)))
  (bind _output_get (Variables|Default|SetHUD _returnvalue))
  (UserInterface|Viewport|AddtoViewport _output_get 0))

(event EventSwapShowAttachmentsMenu
  (bind _hud (Variables|Default|GetHUD))
  (bind _w_attachmentspanel (Variables|/Game/ProWeaponComponent/Blueprints/HUD/Competitive/W_CompetitiveHUD.W_CompetitiveHUD_C|GetW_AttachmentsPanel _hud))
  (Variables|Boolean|SetAttachmentsShowed (not (Variables|Boolean|GetAttachmentsShowed)))
  (Widget|SetVisibility _w_attachmentspanel (select (Variables|Boolean|GetAttachmentsShowed) "Visible" "Hidden"))
  (CallFunction|FocusHUD _w_attachmentspanel))

(event EventUpdate
  (Default|Update (Variables|Default|GetHUD)))

(event EventUpdateWeapons
  (Default|Update (Variables|/Game/ProWeaponComponent/Blueprints/HUD/Competitive/W_CompetitiveHUD.W_CompetitiveHUD_C|GetW_CSWeaponPanel (Variables|Default|GetHUD))))

(event EventSwapShowWeaponsMenu
  (bind _hud (Variables|Default|GetHUD))
  (bind _w_csgoshop (Variables|/Game/ProWeaponComponent/Blueprints/HUD/Competitive/W_CompetitiveHUD.W_CompetitiveHUD_C|GetW_CSGOShop _hud))
  (Variables|Boolean|SetbWeaponsMenuShowed (not (Variables|Boolean|GetbWeaponsMenuShowed)))
  (Widget|SetVisibility _w_csgoshop (select (Variables|Boolean|GetbWeaponsMenuShowed) "Visible" "Hidden"))
  (CallFunction|FocusHUD _w_csgoshop))

(fn ConstructionScript)

(fn FocusHUD
  (params (InWidgetToFocus :type Widget%20Object%20Reference))
  (bind _returnvalue (Game|GetPlayerController 0))
  (bind _attachmentsshowed (Variables|Boolean|GetAttachmentsShowed))
  (bind _bweaponsmenushowed (Variables|Boolean|GetbWeaponsMenuShowed))
  (bind _returnvalue_2 (or _attachmentsshowed _bweaponsmenushowed))
  (Variables|/Script/Engine.PlayerController|SetbShowMouseCursor _returnvalue _returnvalue_2)
  (if _returnvalue_2
    (Input|SetInputModeGameandUI _returnvalue InWidgetToFocus "LockOnCapture" true)
    (else
      (Input|SetInputModeGameOnly _returnvalue))))

(fn IsinHUD
  (return (or (Variables|Boolean|GetAttachmentsShowed) (Variables|Boolean|GetbWeaponsMenuShowed))))