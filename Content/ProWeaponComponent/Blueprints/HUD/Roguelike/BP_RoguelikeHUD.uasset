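; Roguelike HUD Blueprint that creates the W_RoguelikeHUD widget on BeginPlay and adds it to the viewport.
; A toggle event shows or hides the widget's attachments panel, switching the mouse cursor and input mode between Game and UI and Game Only.
; Update forwards refreshes to the widget, and IsInHUD reports whether the attachments panel is open.
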(event EventBeginPlay
  (bind _returnvalue (UserInterface|CreateWidget "/Game/ProWeaponComponent/Blueprints/HUD/Roguelike/W_RoguelikeHUD.W_RoguelikeHUD_C" (Game|GetPlayerController 0)))
  (bind _output_get (Variables|Default|SetHUD _returnvalue))
  (UserInterface|Viewport|AddtoViewport _output_get 0))

(event EventSwapShowAttachmentsMenu
  (bind _returnvalue (Game|GetPlayerController 0))
  (Variables|Boolean|SetAttachmentsShowed (not (Variables|Boolean|GetAttachmentsShowed)))
  (Widget|SetVisibility (Variables|/Game/ProWeaponComponent/Blueprints/HUD/Roguelike/W_RoguelikeHUD.W_RoguelikeHUD_C|GetW_AttachmentsPanel (Variables|Default|GetHUD)) (select (Variables|Boolean|GetAttachmentsShowed) "Visible" "Hidden"))
  (Variables|/Script/Engine.PlayerController|SetbShowMouseCursor _returnvalue (Variables|Boolean|GetAttachmentsShowed))
  (if (Variables|Boolean|GetAttachmentsShowed)
    (Input|SetInputModeGameandUI _returnvalue 0 "DoNotLock" true)
    (else
      (Input|SetInputModeGameOnly _returnvalue))))

(event EventUpdate
  (Default|Update (Variables|Default|GetHUD)))

(fn ConstructionScript)

(fn IsinHUD
  (return (Variables|Boolean|GetAttachmentsShowed)))